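; Thrown grenade projectile that explodes on a short fixed fuse after Throw launches it, playing sound and particles.
; A sphere trace gathers unique pawns in the hit radius and sends each GrenadeHitMessage with location and damage.
; A second trace gathers physics bodies for outward impulses, though its impulse loop reuses the trace loop's element instead of its own.
; The mesh sphere then hides, and the actor destroys itself after a delay.
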(event `Throw`
  (params (Velocity :type "Vector Structure"))
  (bind _projectile (`self.Projectile`))
  (bind _returnvalue (`SceneComponent.K2_GetComponentLocation` (`self.Sphere`)))
  (bind _returnvalue_2 (`SceneComponent.K2_GetComponentLocation` (`self.Sphere`)))
  (bind _returnvalue_3 (`SceneComponent.K2_GetComponentLocation` (`self.Sphere`)))
  (`ActorComponent.Activate` _projectile false)
  (set `MovementComponent.Velocity` Velocity _projectile)
  (`KismetSystemLibrary.Delay` 1.0)
  (`GameplayStatics.PlaySoundAtLocation` "/Game/Sounds/explosion_Cue.Explosion_Cue" _returnvalue_2 (struct) 1.0 1.0 0.0 null null null)
  (`GameplayStatics.SpawnEmitterAtLocation` "/Game/StarterContent/Particles/P_Explosion.P_Explosion" _returnvalue_2)
  (`|ExecutionSequence`
    (:`then_0`
      (bind (_outhits _returnvalue_4) (`KismetSystemLibrary.SphereTraceMultiForObjects` _returnvalue _returnvalue (`self.RadiusHit`) (`|MakeArray` "ObjectTypeQuery3" :!type "EObjectTypeQuery Enum")))
      (if _returnvalue_4
        (for _array_element _outhits
          (`KismetArrayLibrary.Array_AddUnique` (`self.hit actors`) (`.HitActor` (`GameplayStatics.BreakHitResult` _array_element))))
        (for _array_element_2 (`self.hit actors`)
          (message `/Game/Blueprints/FPS/BPI_Character.GrenadeHit` _array_element_2 _returnvalue (`self.Damage`)))))
    (:`then_1`
      (bind (_outhits_2 _returnvalue_5) (`KismetSystemLibrary.SphereTraceMultiForObjects` _returnvalue_3 _returnvalue_3 (`self.RadiusHitPhysicBody`) (`|MakeArray` "ObjectTypeQuery4" :!type "EObjectTypeQuery Enum")))
      (if _returnvalue_5
        (for _array_element_3 _outhits_2
          (bind (_bblockinghit _binitialoverlap _time _distance _location _impactpoint _normal _impactnormal _physmat _hitactor _hitcomponent) (`GameplayStatics.BreakHitResult` _array_element_3))
          (`KismetArrayLibrary.Array_AddUnique` (`self.hitPhysicBodys`) _hitactor))
        (for _ (`self.hitPhysicBodys`)
          (bind _returnvalue_6 (`self.K2_GetActorLocation` _hitactor))
          (`PrimitiveComponent.AddImpulseAtLocation` _hitcomponent (* (- _returnvalue_6 (`self.K2_GetActorLocation`)) (`self.ForceForHitBody`)) _returnvalue_6 "None"))))
    (:`then_2`
      (`SceneComponent.SetHiddenInGame` (`self.Sphere`) true false)
      (`KismetSystemLibrary.Delay` 1.0)
      (`self.K2_DestroyActor`))))

(fn `UserConstructionScript`)