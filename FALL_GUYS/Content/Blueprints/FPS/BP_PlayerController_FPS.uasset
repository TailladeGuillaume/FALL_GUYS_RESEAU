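; BP_PlayerController_FPS is the FPS player controller that respawns the player's first-person character after death.
; On BeginPlay it caches all BP_SpawnPoint actors in the level.
; Tick polls the pawn's IsDead flag and, after a short delay, calls the server respawn, which destroys the pawn and possesses a new one at a random spawn point.
; Respawn requires at least two spawn points, otherwise it prints an error.
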(event `self.ReceiveBeginPlay`
  (bind _outactors (`GameplayStatics.GetAllActorsOfClass` "/Game/Blueprints/FPS/BP_SpawnPoint.BP_SpawnPoint_C"))
  (for _array_element _outactors
    (`KismetSystemLibrary.PrintString` (`KismetStringLibrary.Concat_StrStr` "FIND SPAWN POINT " (`KismetSystemLibrary.GetDisplayName` _array_element)) true true (struct :`R` 1.0 :`G` 0.570903 :`A` 1.0))
    (set `self.ArraySpawnPoints` _outactors)))

(event `self.ReceiveTick`
  (params (DeltaSeconds :type "Float (single-precision)"))
  (bind _asbp_first_person_character (cast `/Game/Blueprints/FPS/BP_FirstPersonCharacter` (`self.K2_GetPawn`)))
  (if (`/Game/Blueprints/FPS/BP_FirstPersonCharacter.IsDead` _asbp_first_person_character)
    (`KismetSystemLibrary.Delay` 3.0)
    (`self.Server_Respawn`)))

(event `Server_Respawn`
  (bind _arrayspawnpoints (`self.ArraySpawnPoints`))
  (if (> (`KismetArrayLibrary.Array_Length` (`self.ArraySpawnPoints`)) 1)
    (`/Engine/EditorBlueprintResources/StandardMacros.DoOnce` false :!label _label
      (:`Completed`
        (`self.K2_DestroyActor` (`self.K2_GetPawn`))
        (bind _returnvalue (`|SpawnActorFromClass` "/Game/Blueprints/FPS/BP_FirstPersonCharacter.BP_FirstPersonCharacter_C" (`self.GetTransform` (`|GetArrayItem` _arrayspawnpoints (- (`KismetMathLibrary.RandomIntegerInRange` 1 (`KismetArrayLibrary.Array_Length` _arrayspawnpoints)) 1))) "AdjustIfPossibleButAlwaysSpawn" "OverrideRootScale" null null))
        (`self.Possess` _returnvalue)
        (goto _label :!via `Reset`)))
    (else
      (`KismetSystemLibrary.PrintString` "Error BP_PlayerController : il n'y a pas de spawn Point sur la map : quel dommage :-3" true true (struct :`R` 1.0 :`B` 0.019788 :`A` 1.0)))))

(fn `UserConstructionScript`)