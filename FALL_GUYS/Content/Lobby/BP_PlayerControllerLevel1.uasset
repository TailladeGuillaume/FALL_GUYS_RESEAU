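; Player controller for Level 1 that logs its start and hides the mouse cursor on BeginPlay.
; A separate client BeginPlay event creates the lobby menu widget and adds it to the player screen; nothing here calls it.
; The server counterpart is an empty event marked old, with a disconnected copy of the widget logic.
; Debug prints in both client and server graphs still name BP_PlayerControllerLobby.
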(event `self.ReceiveBeginPlay`
  (`KismetSystemLibrary.PrintString` "BP_PlayerControllerLevel1 --> BeginPlay" true true (struct :`R` 1.0 :`B` 0.138458 :`A` 1.0))
  (set `self.bShowMouseCursor` false))

(event `Event_Server_BeginPlay`
  ;[1 0.04047 0] Old
)

(event `Event_Client_BeginPlay`
  (`KismetSystemLibrary.PrintString` "BP_PlayerControllerLobby --> Event_Client_BeginPlay" true true (struct :`G` 0.452515 :`B` 1.0 :`A` 1.0))
  (bind _returnvalue (`|CreateWidget` "/Game/Lobby/UI/LobbyWidgetMenu.LobbyWidgetMenu_C" self))
  (`UserWidget.AddToPlayerScreen` _returnvalue 0))

(fn `UserConstructionScript`)