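; BP_BallGame_SuperGameMode is a game mode for a ball game that handles scoring for two teams.
; Its two increment events each add a point to Team1 or Team2 on CustomGameState and print that team's new score.
; Both then share a short delay before printing the combined score in yellow as debug on-screen text.
; BeginPlay, Tick and the construction script are empty.
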(event `IncrementTeam1_Servor`
  (bind _ascustom_game_state (cast `/Game/Blueprints/CustomGameState` (`GameplayStatics.GetGameState`) :!pure true))
  (bind _team1 (`/Game/Blueprints/CustomGameState.Team1` _ascustom_game_state))
  (bind _result (`/Engine/EditorBlueprintResources/StandardMacros.IncrementInt` _team1)
    (:`  `
      (`KismetSystemLibrary.PrintString` (`KismetStringLibrary.Concat_StrStr` "Score Team 1 = " (`KismetStringLibrary.Conv_IntToString` _result)))
      (`KismetSystemLibrary.Delay` 2.0 :!label _label)
      (`KismetSystemLibrary.PrintString` (`KismetStringLibrary.Concat_StrStr` "Score = " (`KismetStringLibrary.Conv_IntToString` _team1) " : " (`KismetStringLibrary.Conv_IntToString` (`/Game/Blueprints/CustomGameState.Team2` _ascustom_game_state))) true true (struct :`R` 1.0 :`G` 1.0 :`A` 1.0)))))

(event `IncrementTeam2_Servor`
  (bind _result (`/Engine/EditorBlueprintResources/StandardMacros.IncrementInt` (`/Game/Blueprints/CustomGameState.Team2` (cast `/Game/Blueprints/CustomGameState` (`GameplayStatics.GetGameState`) :!pure true)))
    (:`  `
      (`KismetSystemLibrary.PrintString` (`KismetStringLibrary.Concat_StrStr` "Score Team 2 = " (`KismetStringLibrary.Conv_IntToString` _result)))
      (goto _label))))

(fn `UserConstructionScript`)