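; Player controller for the lobby that puts the lobby menu on the player's screen.
; On BeginPlay, the authority side waits half a second, then calls the client begin-play event, which creates the LobbyMenu widget owned by this controller.
; The older server begin-play event is an empty stub, with its LobbyWidgetMenu creation left disconnected.
; Debug prints trace startup.
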(event `self.ReceiveBeginPlay`
  (`KismetSystemLibrary.PrintString` "Hello i am a player controller" true true (struct :`R` 1.0 :`B` 0.138458 :`A` 1.0))
  (`/Engine/EditorBlueprintResources/ActorMacros.Switch Has Authority`
    (:`Authority`
      ;[1 1 1] PENSER AU DELAY
      (`KismetSystemLibrary.Delay` 0.5)
      (`self.Event_Client_BeginPlay`))))

(event `Event_Server_BeginPlay`
  ;[1 0.04047 0] Old
)

(event `Event_Client_BeginPlay`
  (`KismetSystemLibrary.PrintString` "BP_PlayerControllerLobby --> Event_Client_BeginPlay" true true (struct :`G` 0.452515 :`B` 1.0 :`A` 1.0))
  (bind _returnvalue (`|CreateWidget` "/Game/Lobby/UI_Lobby_Advenced/LobbyMenu.LobbyMenu_C" self))
  (`UserWidget.AddToPlayerScreen` _returnvalue 0))

(fn `UserConstructionScript`)