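; BP_Goal is a goal trigger that scores a point when a BP_Ball enters its box.
; On overlap it prints a debug message with its ID, which selects whether Team 1 or Team 2 scores.
; Only the server updates BP_SuperGameMode, then spawns a replacement ball at a hardcoded position and destroys the old one.
; Tick draws the trigger box as a debug shape every frame.
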(event `self.ReceiveTick`
  (params (DeltaSeconds :type "Float (single-precision)"))
  (bind _box (`self.Box`))
  (`KismetSystemLibrary.DrawDebugBox` (`SceneComponent.K2_GetComponentLocation` _box) (`BoxComponent.BoxExtent` _box) (struct :`G` 0.101418 :`B` 1.0 :`A` 1.0) (struct) 0.0 1.0))

(event `self.Box.OnComponentBeginOverlap`
  (params (OverlappedComponent :type "PrimitiveComponent Object Reference") (OtherActor :type "Actor Object Reference") (OtherComp :type "PrimitiveComponent Object Reference") (OtherBodyIndex :type Integer) (bFromSweep :type Boolean) (SweepResult :type "HitResult Structure (by ref)"))
  (bind _id (`self.ID`))
  (bind _asbp_ball (cast `/Game/Blueprints/BP_Ball` OtherActor))
  (`KismetSystemLibrary.PrintString` (`KismetStringLibrary.Concat_StrStr` "BUT je suis la cage avec l'ID : " (`KismetStringLibrary.Conv_IntToString` _id)) true true (struct :`R` 1.0 :`A` 1.0) 5.0)
  (switch `int` _id
    (:`0`
      (`/Engine/EditorBlueprintResources/ActorMacros.Switch Has Authority`
        (:`Authority`
          (`/Game/BP_SuperGameMode.IncrementTeam1_Servor` (cast `/Game/BP_SuperGameMode` (`GameplayStatics.GetGameMode`) :!pure true)))))
    (:`1`
      (`/Engine/EditorBlueprintResources/ActorMacros.Switch Has Authority`
        (:`Authority`
          (`/Game/BP_SuperGameMode.IncrementTeam2_Servor` (cast `/Game/BP_SuperGameMode` (`GameplayStatics.GetGameMode`) :!pure true))))))
  (`|SpawnActorFromClass` "/Game/Blueprints/BP_Ball.BP_Ball_C" (`KismetMathLibrary.MakeTransform` (-260.0 -60.0 820.0) (struct) (2.0 2.0 2.0)) "Undefined" "OverrideRootScale" null null)
  (`self.K2_DestroyActor` _asbp_ball))

(fn `UserConstructionScript`)